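; BP_Grid is the tile grid actor that handles terrain data, tile selection and unit pathfinding.
; It sphere-traces the world into a tile map with ground-type costs, draws debug planes at construction, and spawns BP_GridTile actors on BeginPlay.
; Hovering a tile runs four-way A* with Manhattan heuristic from the selected unit and highlights the path.
; Selecting a tile opens a tower selection widget; a debug pathfinder colors open and closed sets.
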(event Custom|Event_NewTileSelected
  (params (SelectedTile :type BP%20Grid%20Tile%20Object%20Reference))
  (Utilities|IsValid (Variables|Grid|GetSelectedTile)
    (:Is%20Valid
      (Default|EventDeselectTile (Variables|Grid|GetSelectedTile)))
    (:Is%20Not%20Valid
      _))
  (Variables|Grid|SetSelectedTile SelectedTile)
  (bind _returnvalue (UserInterface|CreateWidget "/Game/Blueprints/Towers/TowerSelectionWidget.TowerSelectionWidget_C"))
  (UserInterface|Viewport|AddtoViewport _returnvalue 0))

(event Custom|Event_NewTIleOvered
  (params (OVeredTile :type BP%20Grid%20Tile%20Object%20Reference))
  (bind _playercontroller (Variables|Default|GetPlayerController))
  (bind _selectedunit (Variables|/Game/Blueprints/Controllers/BP_PlayerController.BP_PlayerController_C|GetSelectedUnit _playercontroller))
  (Utilities|IsValid (Variables|Grid|GetOveredTile)
    (:Is%20Valid
      (Default|EventEndOverTile (Variables|Grid|GetOveredTile)))
    (:Is%20Not%20Valid
      _))
  (Variables|Grid|SetOveredTile OVeredTile)
  (Pathfinding|HighlightCurrentPath false)
  (if (Math|Boolean|ANDBoolean (Utilities|IsValid _selectedunit) (Utilities|IsValid (Variables|Grid|GetOveredTile)) (not (Variables|Default|GetbIsAUnitMoving)))
    (Pathfinding|FindPathtoTarget (Variables|/Game/Blueprints/Enemies/BP_Enemy.BP_Enemy_C|GetGridIndex _selectedunit) (Variables|/Game/Blueprints/Grid/BP_GridTile.BP_GridTile_C|GetGridIndex (Variables|Grid|GetOveredTile)))
    (Pathfinding|HighlightCurrentPath true)))

(event Custom|DebugEvent_FindPathToTarget
  (params (DebugStartTile :type Vector%202D%20Structure) (DebugTargetTile :type Vector%202D%20Structure))
  (|CollapsedDebugFindPath DebugStartTile DebugTargetTile))

(event EventBeginPlay
  (Rendering|Debug|FlushPersistentDebugLines)
  (Variables|Grid|SetGridLocation (Transformation|GetWorldLocation (Variables|Default|GetScene)))
  (Grid|GenerateMapDatafromWorld)
  (Grid|SpawnTile true)
  (Variables|Default|SetPlayerController (Variables|Default|GetPlayerController)))

(fn ConstructionScript
  (bind _gridsizeworld (Variables|Grid|GetGridSizeWorld))
  (Rendering|Debug|FlushPersistentDebugLines)
  (Variables|Grid|SetGridLocation (Transformation|GetWorldLocation (Variables|Default|GetScene)))
  (Rendering|Debug|DrawDebugBox (Variables|Grid|GetGridLocation) (Math|Vector|MakeVector (.y _gridsizeworld) (.x _gridsizeworld) 5.0) (Variables|Debug|GetGridBoxColor) "0, 0, 0" 1e+06 1e+01)
  (Rendering|Debug|DrawDebugBox (Grid|GridBottomLeft) (Math|Vector|MakeVector 2e+01 2e+01 2e+01) (Variables|Debug|GetBottomLeftColor) "0, 0, 0" 1e+06 1e+01)
  (Grid|GenerateMapDatafromWorld)
  (Debug|DrawTile))

(fn GridBottomLeft
  (bind _scene (Variables|Default|GetScene))
  (bind _gridsizeworld (Variables|Grid|GetGridSizeWorld))
  ;[1 1 1] Locate the position of the bottom left corner of BP_Grid
  (return (- (- (Variables|Grid|GetGridLocation) (* (Math|Vector|GetRightVector _scene) (.x _gridsizeworld))) (* (Math|Vector|GetForwardVector _scene) (.y _gridsizeworld)))))

(fn GridTileNumber
  (bind _gridsizeworld (Variables|Grid|GetGridSizeWorld))
  (bind _tilesize (Variables|Grid|GetTileSize))
  (bind _returnvalue (/ _gridsizeworld _tilesize))
  ;[1 1 1] Calculate the grid tile number in the 2D array
  (return (- (Math|Float|Round (.x _returnvalue)) 1) (- (Math|Float|Round (.y _returnvalue)) 1)))

(fn MySphereTrace
  (params (Location :type Vector) (TraceChannel :type ETraceTypeQuery%20Enum :default "TraceTypeQuery1"))
  (bind (_outhit _returnvalue) (Collision|SphereTraceByChannel Location Location (- (Variables|Grid|GetTileSize) (Variables|Grid|GetTileSizeMinus)) TraceChannel false 0 "None" true "(R=1.000000,G=0.000000,B=0.000000,A=1.000000)" "(R=0.000000,G=1.000000,B=0.000000,A=1.000000)" 2e+01))
  (return _returnvalue (.hitactor _outhit)))

(fn DrawTile
  (bind _keys (Utilities|Map|Keys (Variables|Grid|GetStruct_Tiles)))
  (for _array_element _keys
    (Debug|MyDrawDebugPlane (.worldlocation (.Value (Utilities|Map|Find (Variables|Grid|GetStruct_Tiles) _array_element))) (.groundtype (.Value (Utilities|Map|Find (Variables|Grid|GetStruct_Tiles) _array_element))))))

(fn MyDrawDebugPlane
  (params (Location :type Vector) (GroundType :type Enum_GroundTypes%20Enum :default "NewEnumerator0"))
  (switch Utilities|FlowControl|Switch|SwitchonEnum_GroundTypes GroundType
    (:NewEnumerator0
      (LocalVariables|SetTileColor "(R=0.000000,G=1.000000,B=0.001571,A=1.000000)"))
    (:NewEnumerator1
      (LocalVariables|SetTileColor "(R=0.913490,G=1.000000,B=0.000000,A=1.000000)"))
    (:NewEnumerator2
      (LocalVariables|SetTileColor "(R=0.692708,G=0.303906,B=0.000000,A=1.000000)"))
    (:NewEnumerator3
      (LocalVariables|SetTileColor "(R=1.000000,G=0.024069,B=0.000000,A=1.000000)")))
  (Class|KismetSystemLibrary|DrawDebugPlane (Utilities|Struct|MakePlane (.Z (Math|Vector|BreakVector Location)) 0.0 0.0 1.0) Location (- (Variables|Grid|GetTileSize) (Variables|Grid|GetTileSizeMinus)) (LocalVariables|GetTileColor) 1e+06))

(fn GenerateMapDatafromWorld
  (bind (_gridtilenumberx _gridtilenumbery) (Grid|GridTileNumber))
  (bind _scene (Variables|Default|GetScene))
  (bind _tilesize (Variables|Grid|GetTileSize))
  ;[1 1 1] Set X and Y for all tiles that exist
  (for _index (range 0 _gridtilenumberx)
    (LocalVariables|SetX _index)
    (for _index_2 (range 0 _gridtilenumbery)
      (LocalVariables|SetY _index_2)
      (LocalVariables|SetTilePosition (+ (Grid|GridBottomLeft) (* (Math|Vector|GetRightVector _scene) (+ (* (LocalVariables|GetX) (* _tilesize 2.0)) _tilesize)) (* (Math|Vector|GetForwardVector _scene) (+ (* (LocalVariables|GetY) (* _tilesize 2.0)) _tilesize))))
      ;[1 1 1] Cheack if the tile in TilePosition exists on the ground
      (if (.HitSomething (Grid|MySphereTrace (LocalVariables|GetTilePosition) "TraceTypeQuery3"))
        ;[1 1 1] Check if an obstacle is in TilePosition
        (if (.HitSomething (Grid|MySphereTrace (LocalVariables|GetTilePosition) "TraceTypeQuery4"))
          ;[1 1 1] Set the cost for the tile based on a GroundIndex based on the type of obstacle is on the tile
          (Utilities|Map|Add (Variables|Grid|GetStruct_Tiles) (Math|Vector2D|MakeVector2D (Math|Conversions|ToFloat(Integer) (LocalVariables|GetX)) (Math|Conversions|ToFloat(Integer) (LocalVariables|GetY))) (Utilities|Struct|MakeStruct_Tiles 0 0 (Variables|/Game/Blueprints/Grid/BP_Base_Obstacle.BP_Base_Obstacle_C|GetEnum_GroundTypes (.AsBP%20Base%20Obstacle (Utilities|Casting|CastToBP_Base_Obstacle (.Actor (Grid|MySphereTrace (LocalVariables|GetTilePosition) "TraceTypeQuery4"))))) (LocalVariables|GetTilePosition) (Math|Vector2D|MakeVector2D (Math|Conversions|ToFloat(Integer) (LocalVariables|GetX)) (Math|Conversions|ToFloat(Integer) (LocalVariables|GetY))) (Grid|GetTileCost (Variables|/Game/Blueprints/Grid/BP_Base_Obstacle.BP_Base_Obstacle_C|GetEnum_GroundTypes (.AsBP%20Base%20Obstacle (Utilities|Casting|CastToBP_Base_Obstacle (.Actor (Grid|MySphereTrace (LocalVariables|GetTilePosition) "TraceTypeQuery4")))))) 0 0 0 "(X=0.000000,Y=0.000000)"))
          (else
            ;[1 1 1] Set the cost for the tile based on a GroundIndex of type Normal
            (Utilities|Map|Add (Variables|Grid|GetStruct_Tiles) (Math|Vector2D|MakeVector2D (Math|Conversions|ToFloat(Integer) (LocalVariables|GetX)) (Math|Conversions|ToFloat(Integer) (LocalVariables|GetY))) (Utilities|Struct|MakeStruct_Tiles 0 0 "NewEnumerator0" (LocalVariables|GetTilePosition) (Math|Vector2D|MakeVector2D (Math|Conversions|ToFloat(Integer) (LocalVariables|GetX)) (Math|Conversions|ToFloat(Integer) (LocalVariables|GetY))) (Grid|GetTileCost "NewEnumerator0") 0 0 0 "(X=0.000000,Y=0.000000)"))))
        (else
          ;[1 1 1] Set the cost for the tile based on a GroundIndex of type None
          (Utilities|Map|Add (Variables|Grid|GetStruct_Tiles) (Math|Vector2D|MakeVector2D (Math|Conversions|ToFloat(Integer) (LocalVariables|GetX)) (Math|Conversions|ToFloat(Integer) (LocalVariables|GetY))) (Utilities|Struct|MakeStruct_Tiles 0 0 "NewEnumerator4" (LocalVariables|GetTilePosition) (Math|Vector2D|MakeVector2D (Math|Conversions|ToFloat(Integer) (LocalVariables|GetX)) (Math|Conversions|ToFloat(Integer) (LocalVariables|GetY))) (Grid|GetTileCost "NewEnumerator4") 0 0 0 "(X=0.000000,Y=0.000000)")))))))

(fn SpawnTile
  (params (bSpawnNoneTile :type Boolean))
  (bind _struct_tiles (Variables|Grid|GetStruct_Tiles))
  (bind _keys (Utilities|Map|Keys _struct_tiles))
  (for _array_element _keys
    (if (or (Utilities|Enum|NotEqual(Enum) (.groundtype (.Value (Utilities|Map|Find _struct_tiles _array_element))) "NewEnumerator0") bSpawnNoneTile)
      (bind _returnvalue (Game|SpawnActorfromClass "/Game/Blueprints/Grid/BP_GridTile.BP_GridTile_C" (Math|Conversions|ToTransform(Vector) (.worldlocation (.Value (Utilities|Map|Find _struct_tiles _array_element)))) "Undefined" 0 0))
      (Variables|/Game/Blueprints/Grid/BP_GridTile.BP_GridTile_C|SetGridIndex _returnvalue _array_element)
      (Variables|/Game/Blueprints/Grid/BP_GridTile.BP_GridTile_C|SetBP_Grid _returnvalue self)
      (Utilities|Map|Add _struct_tiles _array_element (Utilities|Struct|MakeStruct_Tiles _returnvalue 0 (.groundtype (.Value (Utilities|Map|Find _struct_tiles _array_element))) (.worldlocation (.Value (Utilities|Map|Find _struct_tiles _array_element))) (.gridindex (.Value (Utilities|Map|Find _struct_tiles _array_element))) (.tilecost (.Value (Utilities|Map|Find _struct_tiles _array_element))) (.finalcost (.Value (Utilities|Map|Find _struct_tiles _array_element))) (.costfromstart (.Value (Utilities|Map|Find _struct_tiles _array_element))) (.estimatedcosttotarget (.Value (Utilities|Map|Find _struct_tiles _array_element))) (.previoustile (.Value (Utilities|Map|Find _struct_tiles _array_element))))))))

(fn GetTileCost
  (params (GridIndex :type Enum_GroundTypes%20Enum :default "NewEnumerator0"))
  ;[1 1 1] Set and return the value of TileCost based on GroundType passed with the call to the function
  (switch Utilities|FlowControl|Switch|SwitchonEnum_GroundTypes GridIndex
    (:NewEnumerator0
      (LocalVariables|SetCost 1))
    (:NewEnumerator1
      (LocalVariables|SetCost 2))
    (:NewEnumerator2
      (LocalVariables|SetCost 5))
    (:NewEnumerator3
      (LocalVariables|SetCost 999 :!label _label))
    (:NewEnumerator4
      (goto _label)))
  (return (LocalVariables|GetCost)))

(fn GetTileNeighbors
  (params (GridIndex :type Vector%202D%20Structure))
  (bind _output_get (LocalVariables|SetPossibleNeighbors (Utilities|Array|MakeArray "(X=1.000000,Y=0.000000)" "(X=0.000000,Y=1.000000)" "(X=-1.000000,Y=0.000000)" "(X=0.000000,Y=-1.000000)")))
  (for _array_element _output_get
    (if (.ReturnValue (Utilities|Map|Find (Variables|Grid|GetStruct_Tiles) (+ _array_element GridIndex)))
      (if (Math|Boolean|ANDBoolean (Utilities|Enum|NotEqual(Enum) (.groundtype (.Value (Utilities|Map|Find (Variables|Grid|GetStruct_Tiles) (+ _array_element GridIndex)))) "NewEnumerator4") (Utilities|Enum|NotEqual(Enum) (.groundtype (.Value (Utilities|Map|Find (Variables|Grid|GetStruct_Tiles) (+ _array_element GridIndex)))) "NewEnumerator3") (== (.unitonthistile (.Value (Utilities|Map|Find (Variables|Grid|GetStruct_Tiles) (+ _array_element GridIndex)))) 0))
        (Utilities|Array|AddUnique (LocalVariables|GetOutNeighbors) (+ _array_element GridIndex)))))
  (return (LocalVariables|GetOutNeighbors)))

(fn GetEstimatedCosttoTarget
  (params (CurrentTile :type Vector%202D%20Structure) (TargetTile :type Vector%202D%20Structure))
  (bind _returnvalue (- CurrentTile TargetTile))
  ;[1 1 1] Calculate the cost to move from SelectedTile to TargetTile
  (return (Math|Float|Round (+ (Math|Float|Absolute(Float) (.x _returnvalue)) (Math|Float|Absolute(Float) (.y _returnvalue))))))

(fn FindPathtoTarget
  (params (StartTile :type Vector%202D%20Structure) (TargetTile :type Vector%202D%20Structure))
  (bind _struct_tiles (Variables|Grid|GetStruct_Tiles))
  (bind _struct_tiles_2 (Variables|Grid|GetStruct_Tiles))
  (bind _struct_tiles_3 (Variables|Grid|GetStruct_Tiles))
  (bind _struct_tiles_4 (Variables|Grid|GetStruct_Tiles))
  (LocalVariables|SetStartTileL StartTile)
  (LocalVariables|SetTargetTileL TargetTile)
  (Utilities|Array|Clear (Variables|Default|GetPath))
  (if (Math|Boolean|ANDBoolean (Utilities|Enum|NotEqual(Enum) (.groundtype (.Value (Utilities|Map|Find (Variables|Grid|GetStruct_Tiles) (LocalVariables|GetTargetTileL)))) "NewEnumerator4") (Utilities|Enum|NotEqual(Enum) (.groundtype (.Value (Utilities|Map|Find (Variables|Grid|GetStruct_Tiles) (LocalVariables|GetTargetTileL)))) "NewEnumerator3") (== (.unitonthistile (.Value (Utilities|Map|Find (Variables|Grid|GetStruct_Tiles) (LocalVariables|GetTargetTileL)))) 0) (.ReturnValue (Utilities|Map|Find (Variables|Grid|GetStruct_Tiles) (LocalVariables|GetTargetTileL))))
    (Utilities|FlowControl|Sequence
      (:then_0
        ;[1 1 1] Default values
        (bind _keys (Utilities|Map|Keys (Variables|Grid|GetStruct_Tiles)))
        (for _array_element _keys
          (Utilities|Map|Add _struct_tiles_4 _array_element (Utilities|Struct|MakeStruct_Tiles (.tileactor (.Value (Utilities|Map|Find _struct_tiles_4 _array_element))) (.unitonthistile (.Value (Utilities|Map|Find _struct_tiles_4 _array_element))) (.groundtype (.Value (Utilities|Map|Find _struct_tiles_4 _array_element))) (.worldlocation (.Value (Utilities|Map|Find _struct_tiles_4 _array_element))) (.gridindex (.Value (Utilities|Map|Find _struct_tiles_4 _array_element))) (.tilecost (.Value (Utilities|Map|Find _struct_tiles_4 _array_element))) 999 999 999 "(X=0.000000,Y=0.000000)")))
        (Utilities|Map|Add _struct_tiles_2 (LocalVariables|GetStartTileL) (Utilities|Struct|MakeStruct_Tiles (.tileactor (.Value (Utilities|Map|Find _struct_tiles_2 (LocalVariables|GetStartTileL)))) (.unitonthistile (.Value (Utilities|Map|Find _struct_tiles_2 (LocalVariables|GetStartTileL)))) (.groundtype (.Value (Utilities|Map|Find _struct_tiles_2 (LocalVariables|GetStartTileL)))) (.worldlocation (.Value (Utilities|Map|Find _struct_tiles_2 (LocalVariables|GetStartTileL)))) (.gridindex (.Value (Utilities|Map|Find _struct_tiles_2 (LocalVariables|GetStartTileL)))) (.tilecost (.Value (Utilities|Map|Find _struct_tiles_2 (LocalVariables|GetStartTileL)))) (Pathfinding|GetEstimatedCosttoTarget (LocalVariables|GetStartTileL) (LocalVariables|GetTargetTileL)) 0 (Pathfinding|GetEstimatedCosttoTarget (LocalVariables|GetStartTileL) (LocalVariables|GetTargetTileL)) "(X=0.000000,Y=0.000000)")))
      (:then_1
        (bind _output_get (LocalVariables|SetCurrentTile (LocalVariables|GetStartTileL)))
        (Utilities|Array|AddUnique (LocalVariables|GetOpenSet) _output_get)
        (while (> (Utilities|Array|Length (LocalVariables|GetOpenSet)) 0)
          (LocalVariables|SetOpenSetCheapest (Utilities|Array|Get(acopy) (LocalVariables|GetOpenSet)))
          (for _array_element_2 (LocalVariables|GetOpenSet)
            ;[1 1 1] Find the cheapest cost to move from StartTile to TargetTile
            (if (< (.finalcost (.Value (Utilities|Map|Find _struct_tiles _array_element_2))) (.finalcost (.Value (Utilities|Map|Find _struct_tiles (LocalVariables|GetOpenSetCheapest)))))
              (LocalVariables|SetOpenSetCheapest _array_element_2 :!label _label)
              (elif (== (.finalcost (.Value (Utilities|Map|Find _struct_tiles _array_element_2))) (.finalcost (.Value (Utilities|Map|Find _struct_tiles (LocalVariables|GetOpenSetCheapest)))))
                (if (< (.estimatedcosttotarget (.Value (Utilities|Map|Find _struct_tiles _array_element_2))) (.estimatedcosttotarget (.Value (Utilities|Map|Find _struct_tiles (LocalVariables|GetOpenSetCheapest)))))
                  (goto _label)))))
          (LocalVariables|SetCurrentTile (LocalVariables|GetOpenSetCheapest))
          (Utilities|Array|RemoveItem (LocalVariables|GetOpenSet) (LocalVariables|GetCurrentTile))
          (Utilities|Array|AddUnique (LocalVariables|GetClosedSet) (LocalVariables|GetCurrentTile))
          (for _array_element_3 (Pathfinding|GetTileNeighbors (LocalVariables|GetCurrentTile))
            (LocalVariables|SetCurrentNeighbor _array_element_3)
            (if (not (Utilities|Array|ContainsItem (LocalVariables|GetClosedSet) (LocalVariables|GetCurrentNeighbor)))
              (LocalVariables|SetCurrentNeighborCostFromStart (+ (.costfromstart (.Value (Utilities|Map|Find (Variables|Grid|GetStruct_Tiles) (LocalVariables|GetCurrentTile)))) (.tilecost (.Value (Utilities|Map|Find _struct_tiles_3 (LocalVariables|GetCurrentNeighbor))))))
              (if (not (Utilities|Array|ContainsItem (LocalVariables|GetOpenSet) (LocalVariables|GetCurrentNeighbor)))
                (Utilities|Array|AddUnique (LocalVariables|GetOpenSet) (LocalVariables|GetCurrentNeighbor))
                (Utilities|Map|Add _struct_tiles_3 (LocalVariables|GetCurrentNeighbor) (Utilities|Struct|MakeStruct_Tiles (.tileactor (.Value (Utilities|Map|Find _struct_tiles_3 (LocalVariables|GetCurrentNeighbor)))) (.unitonthistile (.Value (Utilities|Map|Find _struct_tiles_3 (LocalVariables|GetCurrentNeighbor)))) (.groundtype (.Value (Utilities|Map|Find _struct_tiles_3 (LocalVariables|GetCurrentNeighbor)))) (.worldlocation (.Value (Utilities|Map|Find _struct_tiles_3 (LocalVariables|GetCurrentNeighbor)))) (.gridindex (.Value (Utilities|Map|Find _struct_tiles_3 (LocalVariables|GetCurrentNeighbor)))) (.tilecost (.Value (Utilities|Map|Find _struct_tiles_3 (LocalVariables|GetCurrentNeighbor)))) (+ (Pathfinding|GetEstimatedCosttoTarget (LocalVariables|GetCurrentNeighbor) (LocalVariables|GetTargetTileL)) (LocalVariables|GetCurrentNeighborCostFromStart)) (LocalVariables|GetCurrentNeighborCostFromStart) (Pathfinding|GetEstimatedCosttoTarget (LocalVariables|GetCurrentNeighbor) (LocalVariables|GetTargetTileL)) (LocalVariables|GetCurrentTile)) :!label _label_2)
                (if (Math|Vector|Equal(Vector) (LocalVariables|GetCurrentNeighbor) (LocalVariables|GetTargetTileL) 0.0001)
                  (Variables|Default|SetPath (Pathfinding|RetracePath (LocalVariables|GetTargetTileL) (LocalVariables|GetStartTileL)))
                  (return))
                (elif (< (LocalVariables|GetCurrentNeighborCostFromStart) (.costfromstart (.Value (Utilities|Map|Find _struct_tiles_3 (LocalVariables|GetCurrentNeighbor)))))
                  (goto _label_2))))))
        ;[1 1 1] Fail
        (return)))))

(fn RetracePath
  (params (TargetTile :type Vector%202D%20Structure) (StartTile :type Vector%202D%20Structure))
  (LocalVariables|SetCurrentTIle TargetTile)
  (while (Math|Vector|NotEqual(Vector) (LocalVariables|GetCurrentTIle) StartTile 0.0001)
    (Utilities|Array|AddUnique (LocalVariables|GetInversePath) (LocalVariables|GetCurrentTIle))
    (LocalVariables|SetCurrentTIle (.previoustile (.Value (Utilities|Map|Find (Variables|Grid|GetStruct_Tiles) (LocalVariables|GetCurrentTIle))))))
  (bind _arrayelement (Utilities|Array|ReverseforEachLoop (LocalVariables|GetInversePath))
    (:LoopBody
      (Utilities|Array|AddUnique (LocalVariables|GetOutPath) _arrayelement))
    (:Completed
      (return (LocalVariables|GetOutPath)))))

(fn HighlightCurrentPath
  (params (bIsForHighlight :type Boolean))
  (for _array_element (Variables|Default|GetPath)
    (Utilities|IsValid (.tileactor (.Value (Utilities|Map|Find (Variables|Grid|GetStruct_Tiles) _array_element)))
      (:Is%20Valid
        (Default|EventIsinPath (.tileactor (.Value (Utilities|Map|Find (Variables|Grid|GetStruct_Tiles) _array_element))) bIsForHighlight)))))