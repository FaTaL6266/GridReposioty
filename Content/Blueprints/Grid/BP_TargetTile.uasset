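; BP_TargetTile is a grid marker actor that resolves which tile of BP_Grid it occupies.
; On BeginPlay it finds the grid, then linearly searches StructTiles for the world location closest to itself and stores that key as GridIndex.
; UnitOnThisTile rewrites tile entries in the grid map around a GridIndex update, but its call in SetGridIndex is disconnected.
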(event EventBeginPlay
  (bind _outactors (Actor|GetAllActorsOfClass "/Game/Blueprints/Grid/BP_Grid.BP_Grid_C"))
  (Variables|Default|SetGrid (Utilities|Array|Get(acopy) _outactors))
  (CallFunction|SetGridIndex))

(fn ConstructionScript)

(fn SetGridIndex
  (LocalVariables|SetClosestDistance 1e+10)
  (bind _keys (Utilities|Map|Keys (Variables|/Game/Blueprints/Grid/BP_Grid.BP_Grid_C|GetStruct_Tiles (Variables|Default|GetGrid))))
  (for _array_element _keys
    (if (< (Math|Vector|VectorLength (- (.worldlocation (.Value (Utilities|Map|Find (Variables|/Game/Blueprints/Grid/BP_Grid.BP_Grid_C|GetStruct_Tiles (Variables|Default|GetGrid)) _array_element))) (Transformation|GetActorLocation self))) (LocalVariables|GetClosestDistance))
      (LocalVariables|SetClosestDistance (Math|Vector|VectorLength (- (.worldlocation (.Value (Utilities|Map|Find (Variables|/Game/Blueprints/Grid/BP_Grid.BP_Grid_C|GetStruct_Tiles (Variables|Default|GetGrid)) _array_element))) (Transformation|GetActorLocation self))))
      (LocalVariables|SetClosestIndex _array_element)))
  (Variables|Default|SetGridIndex (LocalVariables|GetClosestIndex)))

(fn UnitonThisTile
  (params (GridIndex :type Vector%202D%20Structure))
  (bind _grid (Variables|Default|GetGrid))
  (bind _grid_2 (Variables|Default|GetGrid))
  (bind _struct_tiles (Variables|/Game/Blueprints/Grid/BP_Grid.BP_Grid_C|GetStruct_Tiles _grid))
  (bind _struct_tiles_2 (Variables|/Game/Blueprints/Grid/BP_Grid.BP_Grid_C|GetStruct_Tiles _grid_2))
  (Utilities|Map|Add _struct_tiles_2 (Variables|Default|GetGridIndex) (Utilities|Struct|MakeStruct_Tiles (.tileactor (.Value (Utilities|Map|Find _struct_tiles_2 (Variables|Default|GetGridIndex)))) 0 (.groundtype (.Value (Utilities|Map|Find _struct_tiles_2 (Variables|Default|GetGridIndex)))) (.worldlocation (.Value (Utilities|Map|Find _struct_tiles_2 (Variables|Default|GetGridIndex)))) (.gridindex (.Value (Utilities|Map|Find _struct_tiles_2 (Variables|Default|GetGridIndex)))) (.tilecost (.Value (Utilities|Map|Find _struct_tiles_2 (Variables|Default|GetGridIndex)))) (.finalcost (.Value (Utilities|Map|Find _struct_tiles_2 (Variables|Default|GetGridIndex)))) (.costfromstart (.Value (Utilities|Map|Find _struct_tiles_2 (Variables|Default|GetGridIndex)))) (.estimatedcosttotarget (.Value (Utilities|Map|Find _struct_tiles_2 (Variables|Default|GetGridIndex)))) (.previoustile (.Value (Utilities|Map|Find _struct_tiles_2 (Variables|Default|GetGridIndex))))))
  (Variables|Default|SetGridIndex GridIndex)
  (Utilities|Map|Add _struct_tiles (Variables|Default|GetGridIndex) (Utilities|Struct|MakeStruct_Tiles (.tileactor (.Value (Utilities|Map|Find _struct_tiles (Variables|Default|GetGridIndex)))) 0 (.groundtype (.Value (Utilities|Map|Find _struct_tiles (Variables|Default|GetGridIndex)))) (.worldlocation (.Value (Utilities|Map|Find _struct_tiles (Variables|Default|GetGridIndex)))) (.gridindex (.Value (Utilities|Map|Find _struct_tiles (Variables|Default|GetGridIndex)))) (.tilecost (.Value (Utilities|Map|Find _struct_tiles (Variables|Default|GetGridIndex)))) (.finalcost (.Value (Utilities|Map|Find _struct_tiles (Variables|Default|GetGridIndex)))) (.costfromstart (.Value (Utilities|Map|Find _struct_tiles (Variables|Default|GetGridIndex)))) (.estimatedcosttotarget (.Value (Utilities|Map|Find _struct_tiles (Variables|Default|GetGridIndex)))) (.previoustile (.Value (Utilities|Map|Find _struct_tiles (Variables|Default|GetGridIndex)))))))