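; Camera pawn that pans across the play area with WASD while keeping the mouse cursor visible.
; Tick polls the keys into horizontal and vertical pan values, scales them by PanningSpeed without delta time, and moves the actor.
; X and Y are clamped using values that BeginPlay reads from the first BP_Clamp actor in the level, while Z stays unchanged.
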(event EventBeginPlay
  ;[1 1 1] Sets the valid play area for the game based on inworld location set by the clamp values
  (bind _outactors (Actor|GetAllActorsOfClass "/Game/Blueprints/Controllers/BP_Clamp.BP_Clamp_C"))
  (Variables|Clamp|Set-XFloat (.X (Math|Vector|BreakVector (Variables|/Game/Blueprints/Controllers/BP_Clamp.BP_Clamp_C|Get-XClamp (Utilities|Array|Get(acopy) _outactors)))))
  (Variables|Clamp|Set+XFloat (.X (Math|Vector|BreakVector (Variables|/Game/Blueprints/Controllers/BP_Clamp.BP_Clamp_C|Get+XClamp (Utilities|Array|Get(acopy) _outactors)))))
  (Variables|Clamp|Set-YFloat (.Y (Math|Vector|BreakVector (Variables|/Game/Blueprints/Controllers/BP_Clamp.BP_Clamp_C|Get-YClamp (Utilities|Array|Get(acopy) _outactors)))))
  (Variables|Clamp|Set+YFloat (.Y (Math|Vector|BreakVector (Variables|/Game/Blueprints/Controllers/BP_Clamp.BP_Clamp_C|Get+YClamp (Utilities|Array|Get(acopy) _outactors))))))

(event EventTick
  (params (DeltaSeconds :type Float%20%28single-precision%29))
  (bind _returnvalue (Game|GetPlayerController 0))
  (bind _panningspeed (Variables|Movement|GetPanningSpeed))
  ;[1 1 1] Camera movement based on user input using WASD.
  ;;[1 1 1] Makes the cursor visible during play.
  (Variables|/Script/Engine.PlayerController|SetbShowMouseCursor (Game|GetPlayerController 0) true)
  ;;[1 1 1] Sets the movement values based on user input.
  ;;;[1 1 1] Determines if the camera should move left or right based on user input.
  (if (Game|Player|IsInputKeyDown _returnvalue "D")
    (Variables|Movement|SetHorizontalPan 1)
    (elif (Game|Player|IsInputKeyDown _returnvalue "A")
      (Variables|Movement|SetHorizontalPan -1)
      (else
        (Variables|Movement|SetHorizontalPan 0))))
  ;;;[1 1 1] Determines if the camera should move up or down based on user input.
  (if (Game|Player|IsInputKeyDown _returnvalue "W")
    (Variables|Movement|SetVerticalPan 1)
    (elif (Game|Player|IsInputKeyDown _returnvalue "S")
      (Variables|Movement|SetVerticalPan -1)
      (else
        (Variables|Movement|SetVerticalPan 0))))
  ;;[1 1 1] Takes the panning value and if the value of either value is not zero, change the location of the camera.
  (if (or (!= (Variables|Movement|GetHorizontalPan) 0) (!= (Variables|Movement|GetVerticalPan) 0))
    ;;[1 1 1] Set the new location of the camera based on user input within the allowed play area.
    (Transformation|SetActorLocation (Math|Vector|MakeVector (Math|Float|Clamp(Float) (.X (Math|Vector|BreakVector (+ (Transformation|GetActorLocation) (Math|Vector|MakeVector (* (Variables|Movement|GetVerticalPan) _panningspeed) (* (Variables|Movement|GetHorizontalPan) _panningspeed) 0.0)))) (Variables|Clamp|Get-XFloat) (Variables|Clamp|Get+XFloat)) (Math|Float|Clamp(Float) (.Y (Math|Vector|BreakVector (+ (Transformation|GetActorLocation) (Math|Vector|MakeVector (* (Variables|Movement|GetVerticalPan) _panningspeed) (* (Variables|Movement|GetHorizontalPan) _panningspeed) 0.0)))) (Variables|Clamp|Get-YFloat) (Variables|Clamp|Get+YFloat)) (.Z (Math|Vector|BreakVector (+ (Transformation|GetActorLocation) (Math|Vector|MakeVector (* (Variables|Movement|GetVerticalPan) _panningspeed) (* (Variables|Movement|GetHorizontalPan) _panningspeed) 0.0))))) false false)))

(fn ConstructionScript)