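; Game mode for a tower defense game that tracks the player's lives and money.
; BeginPlay creates the overlay widget and adds it to the viewport.
; Custom events add or subtract money and reduce lives, showing the lose screen widget whenever lives are at or below zero after a reduction.
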(event Custom|LowerLives
  (params (ReduceLivesBy :type Integer))
  (Variables|Default|SetLives (- (Variables|Default|GetLives) ReduceLivesBy))
  (if (<= (Variables|Default|GetLives) 0)
    (bind _returnvalue (UserInterface|CreateWidget "/Game/Blueprints/Controllers/W_LoseScreen.W_LoseScreen_C"))
    (UserInterface|Viewport|AddtoViewport _returnvalue 0)))

(event Custom|IncreaseMoney
  (params (add :type Integer))
  (Variables|Default|SetMoney (+ add (Variables|Default|GetMoney))))

(event Custom|DecreaseMoney
  (params (sub :type Integer))
  (Variables|Default|SetMoney (- (Variables|Default|GetMoney) sub)))

(event EventBeginPlay
  (bind _returnvalue (UserInterface|CreateWidget "/Game/Blueprints/Controllers/OverlayWidget.OverlayWidget_C"))
  (UserInterface|Viewport|AddtoViewport _returnvalue 0))

(fn ConstructionScript)