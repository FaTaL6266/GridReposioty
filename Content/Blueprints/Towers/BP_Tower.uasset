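; Tower defense turret that takes mesh, range, damage and fire rate from StructTower, applied through TowerInit.
; Sphere overlaps set and clear a BP_Enemy target, which Tick faces by yaw and shoots with homing BP_Projectiles, gated by a Reload delay.
; Without a target, Tick runs a sphere trace for the nearest enemy, but ClosestTargetCalculation only assigns None to TempTarget.
; The data table lookup and TowerInit call are unconnected.
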(event OnComponentBeginOverlap(Sphere)
  (params (OverlappedComponent :type Primitive%20Component%20Object%20Reference) (OtherActor :type Actor%20Object%20Reference) (OtherComp :type Primitive%20Component%20Object%20Reference) (OtherBodyIndex :type Integer) (bFromSweep :type Boolean) (SweepResult :type Hit%20Result%20Structure%20%28by%20ref%29))
  ;[1 1 1] Checks for new targets entering the target range of a tower and sets it to be the tower target.
  (Utilities|IsValid (Variables|Default|GetTarget)
    (:Is%20Not%20Valid
      (bind _asbp_enemy (Utilities|Casting|CastToBP_Enemy OtherActor))
      (Variables|Default|SetTarget _asbp_enemy))))

(event OnComponentEndOverlap(Sphere)
  (params (OverlappedComponent :type Primitive%20Component%20Object%20Reference) (OtherActor :type Actor%20Object%20Reference) (OtherComp :type Primitive%20Component%20Object%20Reference) (OtherBodyIndex :type Integer))
  ;[1 1 1] Sets the target of the tower to 'empty' if the tower target leaves the targetting range of the tower and is not destroyed.
  (if (== OtherActor (Variables|Default|GetTarget))
    (Variables|Default|SetTarget 0)))

(event Custom|TowerInit
  (bind _structtower (Variables|Default|GetStructTower))
  (bind (_name _damage _range _firerate _attacktype _splash _splashrange _splashdamage _shootinglocation _cost _mesh) (Utilities|Struct|BreakStruct_Tower _structtower))
  ;[1 1 1] Set the mesh and range of the tower selected by the user
  (Components|StaticMesh|SetStaticMesh (Variables|Default|GetTowerMesh) _mesh)
  (Components|Sphere|SetSphereRadius (Variables|Default|GetSphere) _range true))

(event Custom|Shoot
  (bind _structtower (Variables|Default|GetStructTower))
  (bind (_name _damage _range _firerate _attacktype _splash _splashrange _splashdamage _shootinglocation _cost _mesh _shootingparticle) (Utilities|Struct|BreakStruct_Tower _structtower))
  ;[1 1 1] Spawns an object of type 'Tower Projectile' with a variable 'reload' to determine the delay between spawned objects based on a value from the tower data.
  (Variables|Default|SetReload true)
  (switch Utilities|FlowControl|Switch|SwitchonEnum_AttackTypes _attacktype
    (:NewEnumerator0
      (Game|SpawnActorfromClass "/Game/Blueprints/Towers/BP_Projectile.BP_Projectile_C" (Transformation|GetActorTransform) "AlwaysSpawn" 0 (Variables|Default|GetTarget) _damage _attacktype 0)
      (Effects|SpawnEmitteratLocation _shootingparticle (Transformation|GetActorLocation))
      (Utilities|FlowControl|Delay _firerate)
      (Variables|Default|SetReload false))))

(event Custom|CheckForNewTarget
  (bind _returnvalue (Transformation|GetActorLocation))
  ;[1 1 1] Determines if any targets exist within the range of the tower and sets the tower target to the nearest target if any exists.
  (Variables|Default|SetCheckForTarget true)
  (bind (_outhits _returnvalue_2) (Collision|MultiSphereTraceForObjects _returnvalue (- _returnvalue "0, 0,1.000000") (.Range (Utilities|Struct|BreakStruct_Tower (Variables|Default|GetStructTower))) (Utilities|Array|MakeArray "ObjectTypeQuery3") false 0 "None"))
  (if _returnvalue_2
    (bind _target (CallFunction|ClosestTargetCalculation _outhits))
    (Utilities|IsValid _target
      (:Is%20Valid
        (Variables|Default|SetTarget _target)
        (Utilities|FlowControl|Delay 0.25))
      (:Is%20Not%20Valid
        _)))
  (Variables|Default|SetCheckForTarget false))

(event EventBeginPlay)

(event EventTick
  (params (DeltaSeconds :type Float%20%28single-precision%29))
  ;[1 1 1] Checks for a new enemy within the range of the tower. If an enemy is stored within 'Tower Target,' the 'Shoot' code will be called. If no target is stored in 'Target Tower,' code will be called to search for a new target.
  (Utilities|IsValid (Variables|Default|GetTarget)
    (:Is%20Valid
      (if (Variables|Default|GetReload)
        _
        (else
          (CallFunction|Shoot)))
      (Transformation|SetActorRotation (Math|Rotator|MakeRotator 0.0 0.0 (+ (.Yaw (Math|Rotator|BreakRotator (Math|Rotator|FindLookatRotation (Transformation|GetActorLocation) (Transformation|GetActorLocation (Variables|Default|GetTarget))))) 1.8e+02))))
    (:Is%20Not%20Valid
      (if (not (Variables|Default|GetCheckForTarget))
        (CallFunction|CheckforNewTarget)))))

(fn ConstructionScript)

(fn ClosestTargetCalculation
  (params (HitResults :type Array%20of%20Hit%20Result%20Structures))
  (for _array_element HitResults
    (Utilities|Casting|CastToBP_Enemy (.HitActor (Collision|BreakHitResult _array_element)))
    (Utilities|IsValid (LocalVariables|GetTempTarget)
      (:Is%20Valid
        (if (< (Math|Vector|VectorLength (- (Transformation|GetActorLocation) (Transformation|GetActorLocation (.HitActor (Collision|BreakHitResult _array_element))))) (LocalVariables|GetTempDistance))
          (LocalVariables|SetTempTarget 0)
          (LocalVariables|SetTempDistance (Math|Vector|VectorLength (- (Transformation|GetActorLocation) (Transformation|GetActorLocation (.HitActor (Collision|BreakHitResult _array_element))))))))
      (:Is%20Not%20Valid
        (LocalVariables|SetTempTarget 0)
        (LocalVariables|SetTempDistance (Math|Vector|VectorLength (- (Transformation|GetActorLocation) (Transformation|GetActorLocation (.HitActor (Collision|BreakHitResult _array_element)))))))))
  (return (LocalVariables|GetTempTarget)))