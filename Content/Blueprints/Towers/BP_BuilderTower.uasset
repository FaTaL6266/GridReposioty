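; BP_BuilderTower is a ghost tower that previews placement under the cursor and spawns the real tower.
; Each tick it snaps the cursor hit to a grid and line-traces for pawns there, setting CanBuild and the ghost material.
; PlaceTower checks CanBuild and GameMode money, spawns and initializes BP_Tower from TowerData, deducts the cost, then destroys itself.
; DestroyBuilderTower removes the ghost without building.
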(event Custom|PlaceTower
  (bind _towerdata (Variables|Default|GetTowerData))
  (bind _cost (Utilities|Struct|BreakStruct_Tower _towerdata))
  ;[1 1 1] Places a tower based on user input in a location if 'Can Build' is true and the player has enough money.
  (if (Variables|Default|GetCanBuild)
    (if (>= (Variables|/Game/Blueprints/Controllers/GM_TowerDefense.GM_TowerDefense_C|GetMoney (Variables|References|GetGameMode)) _cost)
      (bind _returnvalue (Game|SpawnActorfromClass "/Game/Blueprints/Towers/BP_Tower.BP_Tower_C" (Transformation|GetActorTransform) "AlwaysSpawn" 0 0))
      (Variables|/Game/Blueprints/Towers/BP_Tower.BP_Tower_C|SetStructTower _returnvalue (Variables|Default|GetTowerData))
      (Default|TowerInit _returnvalue)
      (Default|DecreaseMoney (Variables|References|GetGameMode) _cost)
      (Actor|DestroyActor))))

(event Custom|DestroyBuilderTower
  ;[1 1 1] Removes the BuilderTowerBP when called from the InputAction RightClick Event in PlayerCameraPawn
  (Actor|DestroyActor))

(event EventBeginPlay)

(event Collision|EventActorBeginOverlap
  (params (OtherActor :type Actor%20Object%20Reference)))

(event EventTick
  (params (DeltaSeconds :type Float%20%28single-precision%29))
  (bind _returnvalue (Game|GetPlayerController 0))
  (bind _array (Utilities|Array|MakeArray "ObjectTypeQuery1"))
  (bind _ghostmesh (Variables|Default|GetGhostMesh))
  (bind (_hitresult _returnvalue_2) (Class|PlayerController|GetHitResultUnderCursorforObjects _returnvalue _array true))
  (bind _returnvalue_3 (Rendering|Material|GetMaterial _ghostmesh 0))
  (bind _location (Collision|BreakHitResult _hitresult))
  (bind (_x _y) (Math|Vector|BreakVector _location))
  ;[1 1 1] Creates a semi-transparent 'Ghost Tower' that follows the user's cursor on screen. The ghost tower will appear green if 'Can Build' is true and red if 'Can Build' is false.
  (if _returnvalue_2
    (bind _output_get (Variables|Default|SetSnapLocation (Math|Vector|MakeVector (Math|Float|SnapToGrid(Float) _x 1e+02) (Math|Float|SnapToGrid(Float) _y 1e+02) 0.0)))
    (bind _returnvalue_4 (Collision|LineTraceForObjects (+ _output_get "0, 0,300.000000") _output_get (Utilities|Array|MakeArray "ObjectTypeQuery3") false 0 "ForOneFrame"))
    ;;[1 1 1] 'Can Build' is set based on the results of a line trace.
    (if _returnvalue_4
      (Variables|Default|SetCanBuild false)
      (if (== _returnvalue_3 0)
        _
        (else
          (Rendering|Material|SetMaterial _ghostmesh 0 0)))
      (else
        (Variables|Default|SetCanBuild true)
        (if (== _returnvalue_3 0)
          _
          (else
            (Rendering|Material|SetMaterial _ghostmesh 0 0)))))
    (Transformation|SetActorLocation (Variables|Default|GetSnapLocation) false false)))

(fn ConstructionScript)