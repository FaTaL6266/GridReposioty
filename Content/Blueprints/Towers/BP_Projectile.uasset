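; Tower projectile that homes in on a TargetRunner and damages it on contact.
; Each tick it moves at constant ProjectileSpeed toward the runner's current position, recording that as LastKnownLocation.
; If the runner becomes invalid, it continues to the last known location and destroys itself once close.
; Sphere overlap with the target runner applies Damage and destroys the projectile, ignoring all other actors.
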(event OnComponentBeginOverlap(Sphere)
  (params (OverlappedComponent :type Primitive%20Component%20Object%20Reference) (OtherActor :type Actor%20Object%20Reference) (OtherComp :type Primitive%20Component%20Object%20Reference) (OtherBodyIndex :type Integer) (bFromSweep :type Boolean) (SweepResult :type Hit%20Result%20Structure%20%28by%20ref%29))
  (bind _targetrunner (Variables|Default|GetTargetRunner))
  ;[1 1 1] When the target is within range of the projectile, damage is applied to the target and the projectile is destroyed.
  (if (== OtherActor _targetrunner)
    (Game|Damage|ApplyDamage _targetrunner (Variables|Default|GetDamage) 0 0)
    (Actor|DestroyActor)))

(event EventTick
  (params (DeltaSeconds :type Float%20%28single-precision%29))
  (bind _targetrunner (Variables|Default|GetTargetRunner))
  (bind _returnvalue (Transformation|GetActorLocation _targetrunner))
  ;[1 1 1] Comment
  (Utilities|IsValid _targetrunner
    (:Is%20Valid
      (Variables|Default|SetLastKnownLocation _returnvalue)
      (Transformation|SetActorLocation (Math|Interpolation|VInterptoConstant (Transformation|GetActorLocation) _returnvalue DeltaSeconds (Variables|Default|GetProjectile%20Speed)) false false))
    (:Is%20Not%20Valid
      (if (< (Math|Vector|VectorLength (- (Transformation|GetActorLocation) (Variables|Default|GetLastKnownLocation))) 1e+01)
        (Actor|DestroyActor)
        (else
          (Transformation|SetActorLocation (Math|Interpolation|VInterptoConstant (Transformation|GetActorLocation) (Variables|Default|GetLastKnownLocation) DeltaSeconds (Variables|Default|GetProjectile%20Speed)) false false))))))

(fn ConstructionScript)