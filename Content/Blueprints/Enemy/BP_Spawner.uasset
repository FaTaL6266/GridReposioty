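; Enemy spawner actor that snaps to the grid and spawns waves of BP_Enemy at its own location.
; On BeginPlay it finds BP_Grid, stores the index of the nearest tile and moves itself onto that tile.
; StartWave reads the Data_Wave row named after the current wave number, spawns that row's Enemy1 count all at once, then increments the wave.
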(event Custom|Event_StartWave
  (bind _returnvalue (Utilities|GetDataTableRow "/Game/Blueprints/Enemy/Data_Wave.Data_Wave" (Utilities|String|StringToName (Utilities|String|ToString(Integer) (Variables|Default|GetWave))))
    (:then
      (Variables|Default|SetWaveData _returnvalue)
      (Utilities|FlowControl|Sequence
        (:then_0
          (if (> (.enemy1 (Variables|Default|GetWaveData)) 0)
            (for _index (range 1 (.enemy1 (Variables|Default|GetWaveData)))
              (Game|SpawnActorfromClass "/Game/Blueprints/Enemy/BP_Enemy.BP_Enemy_C" (Transformation|GetActorTransform) "Undefined" 0 0)
              (Development|PrintString "Hello"))))
        (:then_1
          (Math|Integer|IncrementInt (Variables|Default|GetWave)))))))

(event EventBeginPlay
  (bind _outactors (Actor|GetAllActorsOfClass "/Game/Blueprints/Grid/BP_Grid.BP_Grid_C"))
  (Variables|Default|SetGrid (Utilities|Array|Get(acopy) _outactors))
  (CallFunction|SetGridIndexandSnaptoLocation))

(fn ConstructionScript)

(fn SetGridIndexandSnaptoLocation
  (LocalVariables|SetClosestDistance 1e+10)
  (bind _keys (Utilities|Map|Keys (Variables|/Game/Blueprints/Grid/BP_Grid.BP_Grid_C|GetStruct_Tiles (Variables|Default|GetGrid))))
  (for _array_element _keys
    (if (< (Math|Vector|VectorLength (- (.worldlocation (.Value (Utilities|Map|Find (Variables|/Game/Blueprints/Grid/BP_Grid.BP_Grid_C|GetStruct_Tiles (Variables|Default|GetGrid)) _array_element))) (Transformation|GetActorLocation self))) (LocalVariables|GetClosestDistance))
      (LocalVariables|SetClosestDistance (Math|Vector|VectorLength (- (.worldlocation (.Value (Utilities|Map|Find (Variables|/Game/Blueprints/Grid/BP_Grid.BP_Grid_C|GetStruct_Tiles (Variables|Default|GetGrid)) _array_element))) (Transformation|GetActorLocation self))))
      (LocalVariables|SetClosestIndex _array_element)))
  (Variables|Default|SetGridIndex (LocalVariables|GetClosestIndex))
  (Transformation|SetActorLocation (.worldlocation (.Value (Utilities|Map|Find (Variables|/Game/Blueprints/Grid/BP_Grid.BP_Grid_C|GetStruct_Tiles (Variables|Default|GetGrid)) (LocalVariables|GetClosestIndex)))) false false))