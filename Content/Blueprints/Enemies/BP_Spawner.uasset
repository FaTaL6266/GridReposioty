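; Tower-defense wave spawner that snaps to the nearest BP_Grid tile and runs numbered enemy waves from its location.
; NextWave reads the Data_Enemy row named after the wave number and spawns delayed BP_Enemy AI configured from that row.
; A FinishLine component, placed at EndLocation, deducts game-mode lives and destroys enemies that overlap it.
; Tick advances the wave once spawning has finished and AliveRunners is empty, then shows the W_NextWave widget.
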(event OnComponentBeginOverlap(FinishLine)
  (params (OverlappedComponent :type Primitive%20Component%20Object%20Reference) (OtherActor :type Actor%20Object%20Reference) (OtherComp :type Primitive%20Component%20Object%20Reference) (OtherBodyIndex :type Integer) (bFromSweep :type Boolean) (SweepResult :type Hit%20Result%20Structure%20%28by%20ref%29))
  (bind _asbp_enemy (Utilities|Casting|CastToBP_Enemy OtherActor))
  (bind _asgm_tower_defense (Utilities|Casting|CastToGM_TowerDefense (Game|GetGameMode)))
  (Default|LowerLives _asgm_tower_defense (Variables|/Game/Blueprints/Enemies/BP_Enemy.BP_Enemy_C|GetLifeReduction _asbp_enemy))
  (Utilities|Array|RemoveItem (Variables|Default|GetAliveRunners) _asbp_enemy)
  (Actor|DestroyActor _asbp_enemy))

(event Custom|NextWave
  (Variables|Default|SetSpawnCount 1)
  (bind _returnvalue (Utilities|GetDataTableRow "/Game/Blueprints/Enemies/Data_Enemy.Data_Enemy" (Utilities|String|StringToName (Utilities|String|ToString(Integer) (Variables|Default|GetWave))))
    (:then
      (if (> (Variables|Default|GetSpawnCount) (.EnemyCount (Utilities|Struct|BreakStruct_Enemy _returnvalue))) :!label _label
        (Variables|Default|SetInWave true)
        (else
          (bind _returnvalue_2 (AI|SpawnAIFromClass "/Game/Blueprints/Enemies/BP_Enemy.BP_Enemy_C" 0 (Transformation|GetActorLocation) "0, 0, 0" false))
          (bind _asbp_enemy (Utilities|Casting|CastToBP_Enemy _returnvalue_2))
          (Utilities|Array|Add (Variables|Default|GetAliveRunners) _asbp_enemy)
          (Variables|/Game/Blueprints/Enemies/BP_Enemy.BP_Enemy_C|SetSpawner _asbp_enemy self)
          (Variables|/Game/Blueprints/Enemies/BP_Enemy.BP_Enemy_C|SetCurrentHealth _asbp_enemy (.Health (Utilities|Struct|BreakStruct_Enemy _returnvalue)))
          (Variables|/Game/Blueprints/Enemies/BP_Enemy.BP_Enemy_C|SetMaxHealth _asbp_enemy (.Health (Utilities|Struct|BreakStruct_Enemy _returnvalue)))
          (Variables|/Script/Engine.CharacterMovementComponent|SetMaxWalkSpeed (Variables|/Script/Engine.Character|GetCharacterMovement _asbp_enemy) (.RunSpeed (Utilities|Struct|BreakStruct_Enemy _returnvalue)))
          (Variables|/Game/Blueprints/Enemies/BP_Enemy.BP_Enemy_C|SetValue _asbp_enemy (.Value (Utilities|Struct|BreakStruct_Enemy _returnvalue)))
          (Variables|/Game/Blueprints/Enemies/BP_Enemy.BP_Enemy_C|SetLifeReduction _asbp_enemy (.LifeDeduction (Utilities|Struct|BreakStruct_Enemy _returnvalue)))
          (Class|SkinnedMeshComponent|SetSkeletalMesh (Variables|/Script/Engine.Character|GetMesh _asbp_enemy) (.Mesh (Utilities|Struct|BreakStruct_Enemy _returnvalue)) true)
          (Math|Integer|IncrementInt (Variables|Default|GetSpawnCount)
            (:%20%20
              (Utilities|FlowControl|Delay (.SpawnSpeed (Utilities|Struct|BreakStruct_Enemy _returnvalue)))
              (goto _label))))))))

(event EventBeginPlay
  (bind _asbp_player_controller (Utilities|Casting|CastToBP_PlayerController (Game|GetPlayerController 0)))
  (Variables|Default|SetPlayerController _asbp_player_controller)
  (bind _outactors (Actor|GetAllActorsOfClass "/Game/Blueprints/Grid/BP_Grid.BP_Grid_C"))
  (Variables|Default|SetGrid (Utilities|Array|Get(acopy) _outactors))
  (CallFunction|SetGridIndexandSnaptoLocation)
  (CallFunction|SpawnNextWaveWidget))

(event EventTick
  (params (DeltaSeconds :type Float%20%28single-precision%29))
  (if (and (== (Utilities|Array|Length (Variables|Default|GetAliveRunners)) 0) (Variables|Default|GetInWave))
    (Variables|Default|SetInWave false)
    (Math|Integer|IncrementInt (Variables|Default|GetWave)
      (:%20%20
        (CallFunction|SpawnNextWaveWidget)))))

(fn ConstructionScript
  (Transformation|SetRelativeLocation (Variables|Default|GetFinishLine) (Variables|Default|GetEndLocation) false false))

(fn SpawnNextWaveWidget
  (bind _returnvalue (UserInterface|CreateWidget "/Game/Blueprints/Enemies/W_NextWave.W_NextWave_C"))
  (Rendering|Components|TextRender|SetText (Variables|/Game/Blueprints/Enemies/W_NextWave.W_NextWave_C|GetSpawnText _returnvalue) (Utilities|Text|ToText(String) (Utilities|String|Append "Spawn Wave " (Utilities|String|ToString(Integer) (Variables|Default|GetWave)))))
  (Variables|/Game/Blueprints/Enemies/W_NextWave.W_NextWave_C|SetSpawner _returnvalue self)
  (UserInterface|Viewport|AddtoViewport _returnvalue 0))

(fn SetGridIndexandSnaptoLocation
  (LocalVariables|SetClosestDistance 1e+10)
  (bind _keys (Utilities|Map|Keys (Variables|/Game/Blueprints/Grid/BP_Grid.BP_Grid_C|GetStruct_Tiles (Variables|Default|GetGrid))))
  (for _array_element _keys
    (if (< (Math|Vector|VectorLength (- (.worldlocation (.Value (Utilities|Map|Find (Variables|/Game/Blueprints/Grid/BP_Grid.BP_Grid_C|GetStruct_Tiles (Variables|Default|GetGrid)) _array_element))) (Transformation|GetActorLocation self))) (LocalVariables|GetClosestDistance))
      (LocalVariables|SetClosestDistance (Math|Vector|VectorLength (- (.worldlocation (.Value (Utilities|Map|Find (Variables|/Game/Blueprints/Grid/BP_Grid.BP_Grid_C|GetStruct_Tiles (Variables|Default|GetGrid)) _array_element))) (Transformation|GetActorLocation self))))
      (LocalVariables|SetClosestIndex _array_element)))
  (CallFunction|UnitonThisTile (LocalVariables|GetClosestIndex))
  (Transformation|SetActorLocation (.worldlocation (.Value (Utilities|Map|Find (Variables|/Game/Blueprints/Grid/BP_Grid.BP_Grid_C|GetStruct_Tiles (Variables|Default|GetGrid)) (LocalVariables|GetClosestIndex)))) false false))

(fn UnitonThisTile
  (params (GridIndex :type Vector%202D%20Structure))
  (bind _grid (Variables|Default|GetGrid))
  (bind _grid_2 (Variables|Default|GetGrid))
  (bind _struct_tiles (Variables|/Game/Blueprints/Grid/BP_Grid.BP_Grid_C|GetStruct_Tiles _grid))
  (bind _struct_tiles_2 (Variables|/Game/Blueprints/Grid/BP_Grid.BP_Grid_C|GetStruct_Tiles _grid_2))
  (Utilities|Map|Add _struct_tiles_2 (Variables|Default|GetGridIndex) (Utilities|Struct|MakeStruct_Tiles (.tileactor (.Value (Utilities|Map|Find _struct_tiles_2 (Variables|Default|GetGridIndex)))) 0 (.groundtype (.Value (Utilities|Map|Find _struct_tiles_2 (Variables|Default|GetGridIndex)))) (.worldlocation (.Value (Utilities|Map|Find _struct_tiles_2 (Variables|Default|GetGridIndex)))) (.gridindex (.Value (Utilities|Map|Find _struct_tiles_2 (Variables|Default|GetGridIndex)))) (.tilecost (.Value (Utilities|Map|Find _struct_tiles_2 (Variables|Default|GetGridIndex)))) (.finalcost (.Value (Utilities|Map|Find _struct_tiles_2 (Variables|Default|GetGridIndex)))) (.costfromstart (.Value (Utilities|Map|Find _struct_tiles_2 (Variables|Default|GetGridIndex)))) (.estimatedcosttotarget (.Value (Utilities|Map|Find _struct_tiles_2 (Variables|Default|GetGridIndex)))) (.previoustile (.Value (Utilities|Map|Find _struct_tiles_2 (Variables|Default|GetGridIndex))))))
  (Variables|Default|SetGridIndex GridIndex)
  (Utilities|Map|Add _struct_tiles (Variables|Default|GetGridIndex) (Utilities|Struct|MakeStruct_Tiles (.tileactor (.Value (Utilities|Map|Find _struct_tiles (Variables|Default|GetGridIndex)))) 0 (.groundtype (.Value (Utilities|Map|Find _struct_tiles (Variables|Default|GetGridIndex)))) (.worldlocation (.Value (Utilities|Map|Find _struct_tiles (Variables|Default|GetGridIndex)))) (.gridindex (.Value (Utilities|Map|Find _struct_tiles (Variables|Default|GetGridIndex)))) (.tilecost (.Value (Utilities|Map|Find _struct_tiles (Variables|Default|GetGridIndex)))) (.finalcost (.Value (Utilities|Map|Find _struct_tiles (Variables|Default|GetGridIndex)))) (.costfromstart (.Value (Utilities|Map|Find _struct_tiles (Variables|Default|GetGridIndex)))) (.estimatedcosttotarget (.Value (Utilities|Map|Find _struct_tiles (Variables|Default|GetGridIndex)))) (.previoustile (.Value (Utilities|Map|Find _struct_tiles (Variables|Default|GetGridIndex)))))))