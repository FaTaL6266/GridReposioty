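; Tower defense enemy that walks the grid to the first target tile found and hooks itself to its health bar widget.
; After BeginPlay it registers on the nearest tile and requests a path from BP_Grid.
; The path rebuilds the Grid's shared spline, and a timeline moves the enemy along it.
; Damage, death and kill-reward logic is disconnected, so AnyDamage does nothing; selection events only print.
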(event Custom|Event_Selected
  (Development|PrintString "Selected"))

(event Custom|Event_Deselected
  (Development|PrintString "Deselected"))

(event Custom|Event_MoveAlongThePath
  (params (Path :type Array%20of%20Vector%202D%20Structures))
  (bind _grid (Variables|References|GetGrid))
  (bind _spline (Variables|/Game/Blueprints/Grid/BP_Grid.BP_Grid_C|GetSpline _grid))
  (Variables|Default|SetPath Path)
  (Utilities|Array|Insert (Variables|Default|GetPath) (Variables|Default|GetGridIndex))
  (Spline|ClearSplinePoints (Variables|/Game/Blueprints/Grid/BP_Grid.BP_Grid_C|GetSpline (Variables|References|GetGrid)) true)
  (for _array_element (Variables|Default|GetPath)
    (Development|PrintString (Utilities|String|ToString(Vector2d) _array_element))
    (Spline|AddSplinePoint (Variables|/Game/Blueprints/Grid/BP_Grid.BP_Grid_C|GetSpline (Variables|References|GetGrid)) (Math|Vector|MakeVector (.x (.worldlocation (.Value (Utilities|Map|Find (Variables|/Game/Blueprints/Grid/BP_Grid.BP_Grid_C|GetStruct_Tiles (Variables|References|GetGrid)) _array_element)))) (.y (.worldlocation (.Value (Utilities|Map|Find (Variables|/Game/Blueprints/Grid/BP_Grid.BP_Grid_C|GetStruct_Tiles (Variables|References|GetGrid)) _array_element)))) (+ (.z (.worldlocation (.Value (Utilities|Map|Find (Variables|/Game/Blueprints/Grid/BP_Grid.BP_Grid_C|GetStruct_Tiles (Variables|References|GetGrid)) _array_element)))) (Variables|/Script/Engine.CapsuleComponent|GetCapsuleHalfHeight (Variables|Collision|GetCapsuleComponent)))) "World" true))
  (bind _progression (Timeline|MoveAlongThePathTimeline PlayFromStart)
    (:Update
      (Transformation|SetActorTransform self (Math|Transform|MakeTransform (Spline|GetLocationatDistanceAlongSpline _spline (* _progression (Spline|GetSplineLength _spline)) "World") (Spline|GetRotationatDistanceAlongSpline _spline (* _progression (Spline|GetSplineLength _spline)) "World") "1,1,1")))
    (:Finished
      (Development|PrintString "Done Moving"))))

(event Custom|JunkEvent
  (Development|PrintString "Hello"))

(event Game|Damage|EventAnyDamage
  (params (Damage :type Float%20%28single-precision%29) (DamageType :type Damage%20Type%20Object%20Reference) (InstigatedBy :type Controller%20Object%20Reference) (DamageCauser :type Actor%20Object%20Reference))
  ;[1 1 1] When the AIRunner receives damage, the damage is subtracted from the health of the AIRunner. If the health of th AIRunner is equal to or less than 0, the AIRunner is destroyed.
)

(event EventBeginPlay
  (Utilities|FlowControl|Delay 0.2)
  (bind _asw_healh_bar (Utilities|Casting|CastToW_HealhBar (UserInterface|GetUserWidgetObject (Variables|Default|GetWidget))))
  (Variables|/Game/Blueprints/Enemies/W_HealhBar.W_HealhBar_C|SetEnemy _asw_healh_bar self)
  (bind _outactors (Actor|GetAllActorsOfClass "/Game/Blueprints/Grid/BP_TargetTile.BP_TargetTile_C"))
  (Variables|Default|SetTargetTile (Utilities|Array|Get(acopy) _outactors))
  (bind _outactors_2 (Actor|GetAllActorsOfClass "/Game/Blueprints/Grid/BP_Grid.BP_Grid_C"))
  (Variables|References|SetGrid (Utilities|Array|Get(acopy) _outactors_2))
  (CallFunction|SetGridIndex)
  (Development|PrintString (Utilities|String|ToString(Vector2d) (Variables|/Game/Blueprints/Grid/BP_TargetTile.BP_TargetTile_C|GetGridIndex (Variables|Default|GetTargetTile))))
  (bind _path (Default|FindPathtoTarget (Variables|References|GetGrid) (Variables|Default|GetGridIndex) (Variables|/Game/Blueprints/Grid/BP_TargetTile.BP_TargetTile_C|GetGridIndex (Variables|Default|GetTargetTile))))
  (for _array_element _path
    (Development|PrintString (Utilities|String|ToString(Vector2d) _array_element))
    (CallFunction|EventMoveAlongthePath _path)))

(fn ConstructionScript)

(fn SetGridIndex
  (LocalVariables|SetClosestDistance 1e+10)
  (bind _keys (Utilities|Map|Keys (Variables|/Game/Blueprints/Grid/BP_Grid.BP_Grid_C|GetStruct_Tiles (Variables|References|GetGrid))))
  (for _array_element _keys
    (if (< (Math|Vector|VectorLength (- (.worldlocation (.Value (Utilities|Map|Find (Variables|/Game/Blueprints/Grid/BP_Grid.BP_Grid_C|GetStruct_Tiles (Variables|References|GetGrid)) _array_element))) (Transformation|GetActorLocation self))) (LocalVariables|GetClosestDistance))
      (LocalVariables|SetClosestDistance (Math|Vector|VectorLength (- (.worldlocation (.Value (Utilities|Map|Find (Variables|/Game/Blueprints/Grid/BP_Grid.BP_Grid_C|GetStruct_Tiles (Variables|References|GetGrid)) _array_element))) (Transformation|GetActorLocation self))))
      (LocalVariables|SetClosestIndex _array_element)))
  (CallFunction|UnitonThisTile (LocalVariables|GetClosestIndex)))

(fn UnitonThisTile
  (params (GridIndex :type Vector%202D%20Structure))
  (bind _grid (Variables|References|GetGrid))
  (bind _grid_2 (Variables|References|GetGrid))
  (bind _struct_tiles (Variables|/Game/Blueprints/Grid/BP_Grid.BP_Grid_C|GetStruct_Tiles _grid))
  (bind _struct_tiles_2 (Variables|/Game/Blueprints/Grid/BP_Grid.BP_Grid_C|GetStruct_Tiles _grid_2))
  (Utilities|Map|Add _struct_tiles_2 (Variables|Default|GetGridIndex) (Utilities|Struct|MakeStruct_Tiles (.tileactor (.Value (Utilities|Map|Find _struct_tiles_2 (Variables|Default|GetGridIndex)))) 0 (.groundtype (.Value (Utilities|Map|Find _struct_tiles_2 (Variables|Default|GetGridIndex)))) (.worldlocation (.Value (Utilities|Map|Find _struct_tiles_2 (Variables|Default|GetGridIndex)))) (.gridindex (.Value (Utilities|Map|Find _struct_tiles_2 (Variables|Default|GetGridIndex)))) (.tilecost (.Value (Utilities|Map|Find _struct_tiles_2 (Variables|Default|GetGridIndex)))) (.finalcost (.Value (Utilities|Map|Find _struct_tiles_2 (Variables|Default|GetGridIndex)))) (.costfromstart (.Value (Utilities|Map|Find _struct_tiles_2 (Variables|Default|GetGridIndex)))) (.estimatedcosttotarget (.Value (Utilities|Map|Find _struct_tiles_2 (Variables|Default|GetGridIndex)))) (.previoustile (.Value (Utilities|Map|Find _struct_tiles_2 (Variables|Default|GetGridIndex))))))
  (Variables|Default|SetGridIndex GridIndex)
  (Utilities|Map|Add _struct_tiles (Variables|Default|GetGridIndex) (Utilities|Struct|MakeStruct_Tiles (.tileactor (.Value (Utilities|Map|Find _struct_tiles (Variables|Default|GetGridIndex)))) 0 (.groundtype (.Value (Utilities|Map|Find _struct_tiles (Variables|Default|GetGridIndex)))) (.worldlocation (.Value (Utilities|Map|Find _struct_tiles (Variables|Default|GetGridIndex)))) (.gridindex (.Value (Utilities|Map|Find _struct_tiles (Variables|Default|GetGridIndex)))) (.tilecost (.Value (Utilities|Map|Find _struct_tiles (Variables|Default|GetGridIndex)))) (.finalcost (.Value (Utilities|Map|Find _struct_tiles (Variables|Default|GetGridIndex)))) (.costfromstart (.Value (Utilities|Map|Find _struct_tiles (Variables|Default|GetGridIndex)))) (.estimatedcosttotarget (.Value (Utilities|Map|Find _struct_tiles (Variables|Default|GetGridIndex)))) (.previoustile (.Value (Utilities|Map|Find _struct_tiles (Variables|Default|GetGridIndex)))))))